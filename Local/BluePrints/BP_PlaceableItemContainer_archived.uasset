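; Placeable storage container that opens a chest inventory and sizes it on BeginPlay from its item's AnB_Storage data table row.
; When a journey trigger is set, added items or stack changes credit the last interactor's Exiles Journey component, with an extra Siptah event for the fluid press.
; It exposes its inventory for owner-matched aggregation, with authority-set, replicated sharing access that defaults off on placement under no-ownership servers.
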(event `self.InteractableActivate`
  (params (Component :type "PrimitiveComponent Object Reference") (Instigator :type "PlayerController Object Reference") (HitIndex :type Integer) (TriggeredFromRadialWheel :type Boolean))
  (`parent.InteractableActivate` Component Instigator HitIndex false)
  (set `self.InteractingInstigator` Instigator))

(event `self.ReceiveBeginPlay`
  (bind _placeableinventory (`self.PlaceableInventory`))
  (bind _placeableinventory_2 (`self.PlaceableInventory`))
  (`parent.ReceiveBeginPlay`)
  (bind _returnvalue (`|GetDataTableRow` "/Game/Mods/ash_and_blood/DataTables/ControlTables/AnB_Storage.AnB_Storage" (`KismetStringLibrary.Conv_StringToName` (`KismetStringLibrary.Conv_IntToString` (`self.SourceItemTemplateID`))))
    (:`then`
      (`ItemInventory.SetMaxItemCount` _placeableinventory (`.ItemContainerSize_5_0BFB134C414F4EE78B4130BBC02C84E6` (break `/Game/Mods/ash_and_blood/Structs/ST_Storage` _returnvalue))))
    (:`RowNotFound`
      (`ItemInventory.SetMaxItemCount` _placeableinventory 0)))
  (if (!= (`self.JourneyEventTriggerOnStoringItem`) "None")
    (add `ItemInventory.SignalItemAdded` _placeableinventory_2 (delegate `SignalItemAdded_Event_0`))
    (add `ItemInventory.SignalItemIntStatChanged` _placeableinventory_2 (delegate `SignalITemIntStatChanged`))))

(event `SignalITemIntStatChanged`
  (params (item :type "GameItem Object Reference") (statID :type "EItemIntStatID Enum" :default "MaxStackSize") (statValue :type Integer) (deltaValue :type Integer))
  (bind _interactinginstigator (`self.InteractingInstigator`))
  (bind _journeyeventtriggeronstoringitem (`self.JourneyEventTriggerOnStoringItem`))
  (bind _returnvalue (`Controller.K2_GetPawn` _interactinginstigator))
  (bind _returnvalue_2 (`self.GetComponentByClass` _returnvalue "/Game/Systems/Progression/BP_AC_ExilesJourney.BP_AC_ExilesJourney_C"))
  (bind _returnvalue_3 (`self.K2_GetActorLocation` _returnvalue))
  (if (`|EnumEquality` statID "StackSize")
    (`/Engine/EditorBlueprintResources/StandardMacros.IsValid` _interactinginstigator :!label _label
      (:`Is Valid`
        (`/Engine/EditorBlueprintResources/StandardMacros.IsValid` _returnvalue_2
          (:`Is Valid`
            (`ExilesJourneyComponent.AddJourneyEvent` _returnvalue_2 _journeyeventtriggeronstoringitem _returnvalue_3)
            (if (== _journeyeventtriggeronstoringitem "UseFluidPress")
              (`ExilesJourneyComponent.AddJourneyEvent` _returnvalue_2 "Siptah_UseFluidPress" _returnvalue_3))))))))

(event `SignalItemAdded_Event_0`
  (params (index :type Integer) (item :type "GameItem Object Reference") (srcInventory :type "ItemInventory Object Reference") (srcIndex :type Integer))
  (goto _label))

(event `self.RegisterAggregatableInventories`
  (params (Aggregator :type "InventoryAggregator Object Reference"))
  (`InventoryAggregator.AddInventory` Aggregator (`self.PlaceableInventory`) "Available"))

(event `self.BindTo_ShareableInventoryAccessChanged`
  (params (Delegate :type "Delegate (by ref)"))
  (add `self.OnSharingAccessChanged` Delegate))

(event `self.UnbindFrom_ShareableInventoryAccessChanged`
  (params (Delegate :type "Delegate (by ref)"))
  (remove `self.OnSharingAccessChanged` Delegate))

(event `self.SetShareAccess`
  (params (ShareAccess :type "EInventoryShareAccess Enum" :default "Off"))
  (`/Engine/EditorBlueprintResources/ActorMacros.Switch Has Authority`
    (:`Authority`
      (bind _output_get (set `self.InventorySharingAccess` ShareAccess))
      (`self.OnSharingAccessChanged` self self _output_get))))

(event `self.InteractableMenu`
  (params (RadialMenu :type "RadialMenu Object Reference") (HitIndex :type Integer))
  (`parent.InteractableMenu` RadialMenu HitIndex))

(event `self.SetLockedState`
  (params (`New Value` :type Boolean))
  (`parent.SetLockedState` `New Value`))

(fn `ClientGetCraftingGUICenterPanel`
  (params (Instigator :type "PlayerController Object Reference"))
  (returns (ReturnValue :type Name))
  (return "ChestInventory"))

(fn `GetShareableInventories`
  (returns (OutInventories :type "Array of ItemInventory Object Reference"))
  (return (`|MakeArray` (`self.PlaceableInventory`) :!type "ItemInventory Object Reference")))

(fn `GetShareAccess`
  (returns (ReturnValue :type "EInventoryShareAccess Enum"))
  (return (`self.InventorySharingAccess`)))

(fn `InteractableGetUIModuleName`
  (returns (ReturnValue :type Name))
  (return "ContainerInfo"))

(fn `IsAggregatableWith`
  (params (ID :type "UniqueID Object Reference"))
  (returns (ReturnValue :type Boolean))
  (bind _owneruniqueid (`self.OwnerUniqueID`))
  (return (and (== ID _owneruniqueid) (`DreamworldBlueprints.IsValidID` _owneruniqueid))))

(fn `OnPlaced`
  (params (PlacedBy :type "ConanCharacter Object Reference"))
  (if (`ServerSettings.GetNoOwnership` (`|GetServerSettings`))
    (set `self.InventorySharingAccess` "Off"))
  (`parent.OnPlaced` (`local.PlacedBy`)))

(fn `OnRep_InventorySharingAccess`
  (`self.OnSharingAccessChanged` self self (`self.InventorySharingAccess`)))

(fn `UserConstructionScript`
  (`parent.UserConstructionScript`))