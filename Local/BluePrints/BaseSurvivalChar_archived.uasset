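; Base survival character Blueprint, apparently archived, that adds timed KillPlayer handling to death and supports revival.
; KillCharacter prints debug info and calls KillPlayer, shorter for killers flagged by CheckIsNPCMessage, skipping suicides and causeless BasePlayerChar0 damage, then always runs the parent logic.
; ReviveCharacter calls RevivePlayer and restores default movement.
; AddDownTime applies a longer KillPlayer duration, and GetCommunity returns the killer's community.
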(fn `AddDownTime`
  (params (KillerName :type Text) (Killer :type "ConanCharacter Object Reference"))
  (`/Game/Shared/Death/DeathMacro.Kill Player` KillerName Killer 60.0))

(fn `GetCommunity`
  (returns (Community :type Integer))
  (bind _killer (`self.Killer`))
  (`/Engine/EditorBlueprintResources/StandardMacros.IsValid` _killer
    (:`Is Valid`
      (return (`ConanCharacter.Community` _killer)))
    (:`Is Not Valid`
      (return 0))))

(fn `KillCharacter`
  (params (hitLocation :type "EHitlocation Enum" :default "None") (killerNameInput :type "Text (by ref)") (killer :type "ConanCharacter Object Reference") (OverridingCauseOfDeath :type "ECauseOfDeath Structure") (StateChangeDelay :type "Float (single-precision)") (DamageCauser :type "Actor Object Reference"))
  (returns (ReturnValue :type Integer))
  (bind _name (break `ECauseOfDeath` OverridingCauseOfDeath))
  (bind _returnvalue (`KismetSystemLibrary.GetDisplayName` DamageCauser))
  (bind _returnvalue_2 (`KismetStringLibrary.Conv_NameToString` _name))
  (`KismetSystemLibrary.PrintString` (`KismetStringLibrary.Concat_StrStr` "Cuase: " _returnvalue_2 " \nName: " (`KismetTextLibrary.Conv_TextToString` killerNameInput) " \nCauser: " _returnvalue) true true (struct :`G` 0.66 :`B` 1.0 :`A` 1.0) 35.0 _name)
  (if (not (or (`KismetStringLibrary.EqualEqual_StrStr` _returnvalue_2 "Suicide") (and (`KismetStringLibrary.EqualEqual_StrStr` _returnvalue_2) (`KismetStringLibrary.EqualEqual_StrStr` _returnvalue "BasePlayerChar0"))))
    (bind _isnpc (message `/Game/Systems/Interfaces/BaseBPCharInterface.CheckIsNPC` killer))
    (if _isnpc
      (`/Game/Shared/Death/DeathMacro.Kill Player` killerNameInput killer 10.0
        (:`true`
          _))
      (else
        (`/Game/Shared/Death/DeathMacro.Kill Player` killerNameInput killer 30.0
          (:`true`
            _)))))
  (bind _returnvalue_3 (`parent.KillCharacter` hitLocation killerNameInput killer OverridingCauseOfDeath StateChangeDelay DamageCauser))
  (return _returnvalue_3))

(fn `ReviveCharacter`
  (`/Game/Shared/Death/DeathMacro.Revive Player` 0.2)
  (`CharacterMovementComponent.SetDefaultMovementMode` (`self.CharacterMovement`))
  (`KismetSystemLibrary.PrintString` "Movement has been returned theoretically"))

(fn `UserConstructionScript`
  (`parent.UserConstructionScript`))