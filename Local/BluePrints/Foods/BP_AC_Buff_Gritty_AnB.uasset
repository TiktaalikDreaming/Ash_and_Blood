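; Food buff component that temporarily raises the owning character's Grit (stamina attribute) along with maximum stamina.
; On buff start it merges additive stat modifiers: the configured amount to the attribute and ten times that to max stamina.
; On clear it merges the negated amounts to cancel them.
; Name and description show the Grit amount, but their Endurance bonus is fixed text rather than computed from it.
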(event `self.ReceiveBeginPlay`
  (`parent.ReceiveBeginPlay`)
  (set `self.Name` (`|FormatText` "Grit +{0} Bonus Endurance +40" (`self.BuffStatByThisMuch`))))

(event `self.GameplayEffectToApplyOnBuffStart`
  (bind _owningcharacter (`self.OwningCharacter`))
  (`ConanCharacter.AddIntStatModifier` _owningcharacter "AttributeStamina" "Buff" "Add" (`self.BuffStatByThisMuch`) "Merge")
  (`ConanCharacter.AddIntStatModifier` _owningcharacter "StaminaMax" "Buff" "Add" (* (`self.BuffStatByThisMuch`) 10) "Merge"))

(event `self.GameplayEffectToApplyOnBuffCleared`
  (bind _owningcharacter (`self.OwningCharacter`))
  (`ConanCharacter.AddIntStatModifier` _owningcharacter "AttributeStamina" "Buff" "Add" (* (`self.BuffStatByThisMuch`) -1) "Merge")
  (`ConanCharacter.AddIntStatModifier` _owningcharacter "StaminaMax" "Buff" "Add" (* (`self.BuffStatByThisMuch`) -10) "Merge"))

(fn `GetEffectDescription`
  (returns (Description :type Text))
  (return (`|FormatText` "Grit +{0} Bonus Endurance +40" (`self.BuffStatByThisMuch`))))