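; Sugar Rush food buff component that boosts a character's agility weapon damage, Might (displayed as Strength) and max health.
; Buff start merges modifiers into the owning character's stats; clearing merges negated values to undo them.
; Max health scales at ten times the integer buff amount.
; The name and effect description format the damage percentage from its variable but hardcode the Strength and Health bonuses.
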(event `self.ReceiveBeginPlay`
  (`parent.ReceiveBeginPlay`)
  (set `self.Name` (`|FormatText` "Agility Weapon Damage +{0}% Strength +2 Health +20" (* (`self.BuffFloatStatByThisMuch`) 100.0))))

(event `self.GameplayEffectToApplyOnBuffStart`
  (bind _owningcharacter (`self.OwningCharacter`))
  (`ConanCharacter.AddFloatStatModifier` _owningcharacter "BonusAgiWeaponDmg" "Default" "Multiply" (`self.BuffFloatStatByThisMuch`) "Merge")
  (`ConanCharacter.AddIntStatModifier` _owningcharacter "AttributeMight" "Buff" "Add" (`self.BuffStatByThisMuch`) "Merge")
  (`ConanCharacter.AddIntStatModifier` _owningcharacter "HealthMax" "Buff" "Add" (* (`self.BuffStatByThisMuch`) 10) "Merge"))

(event `self.GameplayEffectToApplyOnBuffCleared`
  (bind _owningcharacter (`self.OwningCharacter`))
  (`ConanCharacter.AddFloatStatModifier` _owningcharacter "BonusAgiWeaponDmg" "Default" "Multiply" (* (`self.BuffFloatStatByThisMuch`) -1.0) "Merge")
  (`ConanCharacter.AddIntStatModifier` _owningcharacter "AttributeMight" "Buff" "Add" (* (`self.BuffStatByThisMuch`) -1) "Merge")
  (`ConanCharacter.AddIntStatModifier` _owningcharacter "HealthMax" "Buff" "Add" (* (`self.BuffStatByThisMuch`) -10) "Merge"))

(fn `GetEffectDescription`
  (returns (Description :type Text))
  (return (`|FormatText` "Agility Weapon Damage +{0}% Strength +2 Health +20" (* (`self.BuffFloatStatByThisMuch`) 100.0))))