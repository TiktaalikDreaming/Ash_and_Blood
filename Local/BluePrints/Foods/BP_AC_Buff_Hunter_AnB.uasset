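; Food buff component that temporarily raises the owning character's Stamina and Athleticism stats, shown as Grit and Agility, and boosts stamina regeneration.
; On buff start it adds BuffStatByThisMuch to both stats as merged Buff modifiers and raises the regen modifier by a fixed amount.
; On clear it applies the negated values to undo them.
; The same formatted text supplies the buff's name and effect description.
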(event `self.ReceiveBeginPlay`
  (`parent.ReceiveBeginPlay`)
  (set `self.Name` (`|FormatText` "Grit +{0} Agility +{0} Extra Stamina regen" (`self.BuffStatByThisMuch`))))

(event `self.GameplayEffectToApplyOnBuffStart`
  (bind _owningcharacter (`self.OwningCharacter`))
  (`ConanCharacter.AddIntStatModifier` _owningcharacter "AttributeStamina" "Buff" "Add" (`self.BuffStatByThisMuch`) "Merge")
  (`ConanCharacter.AddIntStatModifier` _owningcharacter "AttributeAthleticism" "Buff" "Add" (`self.BuffStatByThisMuch`) "Merge")
  (`ConanCharacter.AdjustStaminaRegenMod` (`self.OwningCharacter`) 9.0))

(event `self.GameplayEffectToApplyOnBuffCleared`
  (bind _owningcharacter (`self.OwningCharacter`))
  (`ConanCharacter.AddIntStatModifier` _owningcharacter "AttributeStamina" "Buff" "Add" (* (`self.BuffStatByThisMuch`) -1) "Merge")
  (`ConanCharacter.AddIntStatModifier` _owningcharacter "AttributeAthleticism" "Buff" "Add" (* (`self.BuffStatByThisMuch`) -1) "Merge")
  (`ConanCharacter.AdjustStaminaRegenMod` (`self.OwningCharacter`) -9.0))

(fn `GetEffectDescription`
  (returns (Description :type Text))
  (return (`|FormatText` "Grit +{0} Agility +{0} Extra Stamina regen" (`self.BuffStatByThisMuch`))))