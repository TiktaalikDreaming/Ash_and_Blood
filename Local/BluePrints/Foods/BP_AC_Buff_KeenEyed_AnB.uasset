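; Food buff component, Keen-Eyed, that raises the owning character's maximum stamina and speeds up stamina regeneration.
; On buff start it adds a scaled buff amount to the StaminaMax stat and raises the regen modifier.
; On clear it applies the negated values to reverse both changes.
; The display name and effect description are hardcoded text, independent of the configured buff amount.
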(event `self.ReceiveBeginPlay`
  (`parent.ReceiveBeginPlay`)
  (set `self.Name` (`|FormatText` "Stamina +20 faster Stamina recovery ")))

(event `self.GameplayEffectToApplyOnBuffStart`
  (`ConanCharacter.AddIntStatModifier` (`self.OwningCharacter`) "StaminaMax" "Buff" "Add" (* (`self.BuffStatByThisMuch`) 10) "Merge")
  (`ConanCharacter.AdjustStaminaRegenMod` (`self.OwningCharacter`) 9.0))

(event `self.GameplayEffectToApplyOnBuffCleared`
  (`ConanCharacter.AddIntStatModifier` (`self.OwningCharacter`) "StaminaMax" "Buff" "Add" (* (`self.BuffStatByThisMuch`) -10) "Merge")
  (`ConanCharacter.AdjustStaminaRegenMod` (`self.OwningCharacter`) -9.0))

(fn `GetEffectDescription`
  (returns (Description :type Text))
  (return (`|FormatText` "Stamina +20 faster Stamina recovery ")))