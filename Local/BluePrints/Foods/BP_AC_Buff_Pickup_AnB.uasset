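; Food buff component that temporarily raises the owning character's Vitality (AttributeHealth) and maximum health.
; On buff start it merges additive stat modifiers, with max health scaled at ten times the configurable buff amount.
; On clear it merges the negated amounts to cancel them.
; The display name and effect description show the Vitality amount but hardcode the bonus health figure rather than deriving it.
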(event `self.ReceiveBeginPlay`
  (`parent.ReceiveBeginPlay`)
  (set `self.Name` (`|FormatText` "Vitality +{0} Bonus Health +20" (`self.BuffStatByThisMuch`))))

(event `self.GameplayEffectToApplyOnBuffStart`
  (bind _owningcharacter (`self.OwningCharacter`))
  (`ConanCharacter.AddIntStatModifier` _owningcharacter "AttributeHealth" "Buff" "Add" (`self.BuffStatByThisMuch`) "Merge")
  (`ConanCharacter.AddIntStatModifier` _owningcharacter "HealthMax" "Buff" "Add" (* (`self.BuffStatByThisMuch`) 10) "Merge"))

(event `self.GameplayEffectToApplyOnBuffCleared`
  (bind _owningcharacter (`self.OwningCharacter`))
  (`ConanCharacter.AddIntStatModifier` _owningcharacter "AttributeHealth" "Buff" "Add" (* (`self.BuffStatByThisMuch`) -1) "Merge")
  (`ConanCharacter.AddIntStatModifier` _owningcharacter "HealthMax" "Buff" "Add" (* (`self.BuffStatByThisMuch`) -10) "Merge"))

(fn `GetEffectDescription`
  (returns (Description :type Text))
  (return (`|FormatText` "Vitality +{0} Bonus Health +20" (`self.BuffStatByThisMuch`))))