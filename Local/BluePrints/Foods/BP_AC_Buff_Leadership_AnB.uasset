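; Food buff component that temporarily raises the owning character's follower damage, concussive damage and Leadership (shown as Authority).
; On buff start it merges multiplicative float modifiers and an additive integer modifier into the character's stats.
; On clear it merges the negated values to undo them.
; Name and description show the follower damage percentage, with the Authority bonus hardcoded and concussive damage unlisted.
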(event `self.ReceiveBeginPlay`
  (`parent.ReceiveBeginPlay`)
  (set `self.Name` (`|FormatText` "Follower Damage +{0}% Bonus Authority +4" (* (`self.BuffFloatStatByThisMuch`) 100.0))))

(event `self.GameplayEffectToApplyOnBuffStart`
  (bind _bufffloatstatbythismuch (`self.BuffFloatStatByThisMuch`))
  (bind _owningcharacter (`self.OwningCharacter`))
  (`ConanCharacter.AddFloatStatModifier` _owningcharacter "BonusFollowerDamage" "Default" "Multiply" _bufffloatstatbythismuch "Merge")
  (`ConanCharacter.AddFloatStatModifier` _owningcharacter "BonusConcussiveDamage" "Default" "Multiply" _bufffloatstatbythismuch "Merge")
  (`ConanCharacter.AddIntStatModifier` _owningcharacter "AttributeLeadership" "Buff" "Add" (`self.BuffStatByThisMuch`) "Merge"))

(event `self.GameplayEffectToApplyOnBuffCleared`
  (bind _owningcharacter (`self.OwningCharacter`))
  (bind _returnvalue (* (`self.BuffFloatStatByThisMuch`) -1.0))
  (`ConanCharacter.AddFloatStatModifier` _owningcharacter "BonusFollowerDamage" "Default" "Multiply" _returnvalue "Merge")
  (`ConanCharacter.AddFloatStatModifier` _owningcharacter "BonusConcussiveDamage" "Default" "Multiply" _returnvalue "Merge")
  (`ConanCharacter.AddIntStatModifier` _owningcharacter "AttributeLeadership" "Buff" "Add" (* (`self.BuffStatByThisMuch`) -1) "Merge"))

(fn `GetEffectDescription`
  (returns (Description :type Text))
  (return (`|FormatText` "Follower Damage +{0}% Bonus Authority +4" (* (`self.BuffFloatStatByThisMuch`) 100.0))))