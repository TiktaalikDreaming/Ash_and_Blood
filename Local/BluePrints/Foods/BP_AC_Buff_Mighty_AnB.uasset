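; Mighty food buff component that temporarily raises the owning character's strength weapon damage and Might attribute.
; On buff start it merges a multiply float modifier and an additive int modifier into the character's stats, then merges negated values when cleared.
; BeginPlay and GetEffectDescription build the same text from the damage percentage, with the +4 Strength bonus hard-coded rather than read from the buff value.
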(event `self.ReceiveBeginPlay`
  (`parent.ReceiveBeginPlay`)
  (set `self.Name` (`|FormatText` "Strength Weapon Damage +{0}% Bonus Strength +4" (* (`self.BuffFloatStatByThisMuch`) 100.0))))

(event `self.GameplayEffectToApplyOnBuffStart`
  (bind _owningcharacter (`self.OwningCharacter`))
  (`ConanCharacter.AddFloatStatModifier` _owningcharacter "BonusStrWeaponDmg" "Default" "Multiply" (`self.BuffFloatStatByThisMuch`) "Merge")
  (`ConanCharacter.AddIntStatModifier` _owningcharacter "AttributeMight" "Buff" "Add" (`self.BuffStatByThisMuch`) "Merge"))

(event `self.GameplayEffectToApplyOnBuffCleared`
  (bind _owningcharacter (`self.OwningCharacter`))
  (`ConanCharacter.AddFloatStatModifier` _owningcharacter "BonusStrWeaponDmg" "Default" "Multiply" (* (`self.BuffFloatStatByThisMuch`) -1.0) "Merge")
  (`ConanCharacter.AddIntStatModifier` _owningcharacter "AttributeMight" "Buff" "Add" (* (`self.BuffStatByThisMuch`) -1) "Merge"))

(fn `GetEffectDescription`
  (returns (Description :type Text))
  (return (`|FormatText` "Strength Weapon Damage +{0}% Bonus Strength +4" (* (`self.BuffFloatStatByThisMuch`) 100.0))))