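; Food buff component "Mule" that temporarily raises the owning character's bonus carry capacity and Encumbrance attribute.
; On buff start it merges additive float and int stat modifiers from the inherited buff amounts, then adds their negatives on clear.
; BeginPlay builds the display name from the carry amount, while GetEffectDescription shows it times 100; both hardcode "Bonus Expertise +4".
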(event `self.ReceiveBeginPlay`
  (`parent.ReceiveBeginPlay`)
  (set `self.Name` (`|FormatText` "Bonus Carry +{0} Bonus Expertise +4" (`self.BuffFloatStatByThisMuch`))))

(event `self.GameplayEffectToApplyOnBuffStart`
  (bind _owningcharacter (`self.OwningCharacter`))
  (`ConanCharacter.AddFloatStatModifier` _owningcharacter "BonusCarryCapacity" "Default" "Add" (`self.BuffFloatStatByThisMuch`) "Merge")
  (`ConanCharacter.AddIntStatModifier` _owningcharacter "AttributeEncumbrance" "Buff" "Add" (`self.BuffStatByThisMuch`) "Merge"))

(event `self.GameplayEffectToApplyOnBuffCleared`
  (bind _owningcharacter (`self.OwningCharacter`))
  (`ConanCharacter.AddFloatStatModifier` _owningcharacter "BonusCarryCapacity" "Default" "Add" (* (`self.BuffFloatStatByThisMuch`) -1.0) "Merge")
  (`ConanCharacter.AddIntStatModifier` _owningcharacter "AttributeEncumbrance" "Buff" "Add" (* (`self.BuffStatByThisMuch`) -1) "Merge"))

(fn `GetEffectDescription`
  (returns (Description :type Text))
  (return (`|FormatText` "Bonus Carry +{0} Bonus Expertise +4" (* (`self.BuffFloatStatByThisMuch`) 100.0))))