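; Food buff component "Hearthy AnB" that boosts the owning character's strength weapon damage and health attribute while active.
; On buff start it merges a multiply modifier for damage and two additive AttributeHealth modifiers, one base and one tenfold.
; On clear it merges the negated values to undo them.
; Name and description format the damage percent but hard-code Vitality +2 and Health +20, though both integer modifiers target AttributeHealth.
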(event `self.ReceiveBeginPlay`
  (`parent.ReceiveBeginPlay`)
  (set `self.Name` (`|FormatText` "Strength Weapon Damage +{0}% Vitality +2 Health +20" (* (`self.BuffFloatStatByThisMuch`) 100.0))))

(event `self.GameplayEffectToApplyOnBuffStart`
  (bind _buffstatbythismuch (`self.BuffStatByThisMuch`))
  (bind _owningcharacter (`self.OwningCharacter`))
  (`ConanCharacter.AddFloatStatModifier` _owningcharacter "BonusStrWeaponDmg" "Default" "Multiply" (`self.BuffFloatStatByThisMuch`) "Merge")
  (`ConanCharacter.AddIntStatModifier` _owningcharacter "AttributeHealth" "Buff" "Add" _buffstatbythismuch "Merge")
  (`ConanCharacter.AddIntStatModifier` _owningcharacter "AttributeHealth" "Buff" "Add" (* _buffstatbythismuch 10) "Merge"))

(event `self.GameplayEffectToApplyOnBuffCleared`
  (bind _owningcharacter (`self.OwningCharacter`))
  (bind _returnvalue (* (`self.BuffStatByThisMuch`) -1))
  (`ConanCharacter.AddFloatStatModifier` _owningcharacter "BonusStrWeaponDmg" "Default" "Multiply" (* (`self.BuffFloatStatByThisMuch`) -1.0) "Merge")
  (`ConanCharacter.AddIntStatModifier` _owningcharacter "AttributeHealth" "Buff" "Add" _returnvalue "Merge")
  (`ConanCharacter.AddIntStatModifier` _owningcharacter "AttributeHealth" "Buff" "Add" (* _returnvalue 10) "Merge"))

(fn `GetEffectDescription`
  (returns (Description :type Text))
  (return (`|FormatText` "Strength Weapon Damage +{0}% Vitality +2 Health +20" (* (`self.BuffFloatStatByThisMuch`) 100.0))))