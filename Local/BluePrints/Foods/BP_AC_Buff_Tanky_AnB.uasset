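; Food buff component that makes the owning character tankier by raising Armor and max health.
; On buff start it merges additive Armor and HealthMax stat modifiers into the owner, then on clear merges the negated amounts to undo them.
; Its name and effect description show the Armor bonus as a percentage from the variable, while the +60 health figure is hardcoded text, independent of the applied value.
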(event `self.ReceiveBeginPlay`
  (`parent.ReceiveBeginPlay`)
  (set `self.Name` (`|FormatText` "Armor +{0}% Bonus Health +60" (* (`self.BuffFloatStatByThisMuch`) 100.0))))

(event `self.GameplayEffectToApplyOnBuffStart`
  (bind _owningcharacter (`self.OwningCharacter`))
  (`ConanCharacter.AddFloatStatModifier` _owningcharacter "Armor" "Default" "Add" (`self.BuffFloatStatByThisMuch`) "Merge")
  (`ConanCharacter.AddIntStatModifier` _owningcharacter "HealthMax" "Buff" "Add" (`self.BuffStatByThisMuch`) "Merge"))

(event `self.GameplayEffectToApplyOnBuffCleared`
  (bind _owningcharacter (`self.OwningCharacter`))
  (`ConanCharacter.AddFloatStatModifier` _owningcharacter "Armor" "Default" "Add" (* (`self.BuffFloatStatByThisMuch`) -1.0) "Merge")
  (`ConanCharacter.AddIntStatModifier` _owningcharacter "HealthMax" "Buff" "Add" (* (`self.BuffStatByThisMuch`) -1) "Merge"))

(fn `GetEffectDescription`
  (returns (Description :type Text))
  (return (`|FormatText` "Armor +{0}% Bonus Health +60" (* (`self.BuffFloatStatByThisMuch`) 100.0))))