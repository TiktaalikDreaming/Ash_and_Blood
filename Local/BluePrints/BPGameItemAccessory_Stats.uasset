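; Conan equippable accessory item, counted as armour, that grants stats and buffs to its wearer.
; On equip and unequip, the authority updates visuals and re-totals armour, knockback defense and climbing stamina cost from equipped BPGameItemArmor items onto BaseBPCombat.
; Buffs apply after a short delay, gated against early unequip, and removal spares buffs other equipped items provide.
; Modkit modifiers write replicated float and int stats on the item.
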(event `self.OnEquip`
  (params (owner :type "Character Object Reference"))
  (bind _returnvalue (`Actor.GetComponentByInterface` owner "/Game/Systems/Buffs/BuffSystemInterface.BuffSystemInterface_C"))
  (`parent.OnEquip` owner)
  (`self.HandleEquip` owner true)
  (add `self.SignalFloatStatChanged` self (`|CreateDelegate` :!event `HandleBroken`))
  (add `self.SignalIntStatChanged` (`|CreateDelegate` :!event `HandleVisualItemChange`))
  (if (> (`KismetArrayLibrary.Array_Length` (`self.Bufflist`)) 0)
    (`|ExecutionSequence`
      (:`then_0`
        (`KismetSystemLibrary.Delay` 0.2)
        (`/Engine/EditorBlueprintResources/StandardMacros.Gate` false :!label _label ; Ensure we haven't un-equipped this item
          (:`Exit`
            (`/Engine/EditorBlueprintResources/StandardMacros.IsValid` _returnvalue
              (:`Is Valid`
                (for _array_element (`self.Bufflist`)
                  (message `/Game/Systems/Buffs/BuffSystemInterface.AddBuffCall` _returnvalue _array_element owner 0 (`Pawn.GetController` owner))))))))
      (:`then_1`
        (goto _label :!via `Open`)))))

(event `self.OnUnEquip`
  (params (owner :type "Character Object Reference"))
  (`parent.OnUnEquip` owner)
  (`self.HandleEquip` owner)
  (remove `self.SignalFloatStatChanged` self (`|CreateDelegate` :!event `HandleBroken`))
  (remove `self.SignalIntStatChanged` (`|CreateDelegate` :!event `HandleVisualItemChange`))
  (if (> (`KismetArrayLibrary.Array_Length` (`self.Bufflist`)) 0)
    (`self.EnsureBuffsRemoved` null)
    (goto _label :!via `Close`)))

(fn `EnsureBuffsRemoved`
  (params (Object :type "Object Object Reference"))
  (locals (BuffsToRemove :type "Array of /Game/Systems/Buffs/01_BP_AC_Buff_Master Class Reference"))
  (bind _asconan_character (cast `ConanCharacter` Object))
  (bind _returnvalue (`ConanCharacter.GetEquipmentInventoryNative` _asconan_character))
  (bind _returnvalue_2 (`Actor.GetComponentByInterface` _asconan_character "/Game/Systems/Buffs/BuffSystemInterface.BuffSystemInterface_C"))
  (`/Engine/EditorBlueprintResources/StandardMacros.IsValid` _returnvalue_2
    (:`Is Valid`
      (`KismetArrayLibrary.Array_Append` (`local.BuffsToRemove`) (`self.Bufflist`))
      (for _array_element (`ItemInventory.ItemList` _returnvalue)
        (bind _asbpgame_item_equipment (cast `/Game/Systems/Inventory/BPGameItemEquipment` _array_element))
        (bind (_arrayindex _arrayelement) (`/Engine/EditorBlueprintResources/StandardMacros.ReverseForEachLoop` (`local.BuffsToRemove`))
          (:`LoopBody`
            (if (`KismetArrayLibrary.Array_Contains` (`/Game/Systems/Inventory/BPGameItemEquipment.Bufflist` _asbpgame_item_equipment) _arrayelement)
              (`KismetArrayLibrary.Array_Remove` (`local.BuffsToRemove`) _arrayindex)))))
      (for _array_element_2 (`local.BuffsToRemove`)
        (message `/Game/Systems/Buffs/BuffSystemInterface.RemoveBuffCall` _returnvalue_2 _array_element_2)))))

(fn `HandleEquip`
  (params (Owner :type "Character Object Reference") (Equip :type Boolean))
  (locals (`local Equip` :type Boolean) (`local ArrayElement` :type "GameItem Object Reference") (`local ArmorValue` :type "Float (double-precision)") (`local KnockbackDefense` :type Integer) (`local ClimbingStaminaCostMod` :type "Float (double-precision)"))
  (set `local.local Equip` Equip)
  (if (`Actor.HasAuthority` Owner)
    (`self.ApplyVisualToChar` (select `bool` (`local.local Equip`) :`false` -1 :`true` (`self.GetVisualItemTemplateId`)))
    (bind _asconan_character (cast `ConanCharacter` (`self.GetOwner`)))
    (bind _returnvalue (`ConanCharacter.GetEquipmentInventoryNative` _asconan_character))
    (for _array_element (`ItemInventory.ItemList` _returnvalue)
      (set `local.local ArrayElement` _array_element)
      (if (`KismetMathLibrary.ClassIsChildOf` (`GameplayStatics.GetObjectClass` (`local.local ArrayElement`)) "/Game/Items/BPGameItemArmor.BPGameItemArmor_C")
        (set `local.local ArmorValue` (+ (`local.local ArmorValue`) (`self.GetFloatStat` (`local.local ArrayElement`) "ArmourValue")))
        (set `local.local KnockbackDefense` (+ (`local.local KnockbackDefense`) (`self.GetIntStat` (`local.local ArrayElement`) "KnockbackDefense")))
        (set `local.local ClimbingStaminaCostMod` (+ (`local.local ClimbingStaminaCostMod`) (`self.GetFloatStat` (`local.local ArrayElement`) "StaminaClimbingCostMultiplier")))))
    (bind _asbase_bpcombat (cast `/Game/Characters/BaseBPCombat` (`self.GetOwner`)))
    (`/Game/Characters/BaseBPCombat.SetArmor` _asbase_bpcombat (`local.local ArmorValue`))
    (`/Game/Characters/BaseBPCombat.SetKnockbackDefense` _asbase_bpcombat (`local.local KnockbackDefense`))
    (`/Game/Characters/BaseBPCombat.SetClimbingStaminaCostModifier` _asbase_bpcombat (`KismetMathLibrary.FMax` (+ (`local.local ClimbingStaminaCostMod`) 1.0)))))

(fn `IsArmour`
  (returns (IsArmour :type Boolean))
  (return true))

(fn `Set Stat Modifiers`
  (params (ModifierInfo :type "/Game/Systems/RiddleOfSteel/RiddleofSteelStruct Structure") (TierMultiplier :type Integer) (RemoveModifiers :type Boolean))
  (locals (LocalModkitInfo :type "/Game/Systems/RiddleOfSteel/RiddleofSteelStruct Structure"))
  (`parent.Set Stat Modifiers` ModifierInfo TierMultiplier RemoveModifiers)
  (bind _output_get (set `local.LocalModkitInfo` ModifierInfo))
  (bind _returnvalue (`self.GetModkitFloatStatModification` _output_get))
  (`self.SetFloatStat` (`.FloatStatModifierType_2_7A305DDD4A9FF72C9B23EEB3369DD4D1` (break `/Game/Systems/RiddleOfSteel/RiddleofSteelStruct` (`local.LocalModkitInfo`))) _returnvalue)
  (bind _returnvalue_2 (`self.GetModkitIntStatModification` (`local.LocalModkitInfo`) TierMultiplier RemoveModifiers))
  (`self.SetIntStat` (`.IntStatModifierType_11_274F1B094CCD56B8FAE58EBD184A0A8E` (break `/Game/Systems/RiddleOfSteel/RiddleofSteelStruct` (`local.LocalModkitInfo`))) _returnvalue_2))