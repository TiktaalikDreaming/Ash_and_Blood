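; Inventory item Blueprint for an equippable accessory, handing equip and unequip to the owner's AC_acs_AccessorySystem component.
; SetData reads the equip location from item stats and the visual-only and any-slot flags from the accessory master DataTable.
; On equip, it packs these with dye channels and rigid attachment into an accessory info struct.
; Parent stat modifiers apply only when AllowStatMods is set, and item-on-item drops are refused.
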(event `self.SetData`
  (params (templateID :type Integer))
  (`parent.SetData` templateID)
  (set `self.EquipmentLocation` (`self.GetIntStat` "EquipLocation"))
  (bind _returnvalue (`|GetDataTableRow` "/Game/ModsShared/AccessorySystem/DataTables/acs_AccessoryDataMasterTable.acs_AccessoryDataMasterTable" (`KismetStringLibrary.Conv_StringToName` (`KismetStringLibrary.Conv_IntToString` (`self.TemplateID`))))
    (:`then`
      (bind ((`AccessoryHiddenUnderArmour_45_0676439C41DA8839EF514285923AD287` _accessoryhiddenunderarmour) (`IsAccessoryVisualOnly?_41_3816585744CE041209A67FA5896399B0` _isaccessoryvisualonly_) (`AllowInUniversalSlots?_46_EA622426414AF7AB7D380581A20F6479` _allowinuniversalslots_)) (break `/Game/ModsShared/AccessorySystem/Structs/ST_acs_AccessoryDataRow` _returnvalue))
      (set `self.VisualOnly` _isaccessoryvisualonly_)
      (set `self.AllowAnySlot` _allowinuniversalslots_))))

(event `self.OnEquip`
  (params (owner :type "Character Object Reference"))
  (`/Game/ModsShared/AccessorySystem/Components/AC_acs_AccessorySystem.EquipAccessory` (`Actor.GetComponentByClass` owner "/Game/ModsShared/AccessorySystem/Components/AC_acs_AccessorySystem.AC_acs_AccessorySystem_C") (`self.MakeAccessoryInfo`)))

(event `self.OnUnEquip`
  (params (owner :type "Character Object Reference"))
  (`/Game/ModsShared/AccessorySystem/Components/AC_acs_AccessorySystem.UnequipAccessory` (`Actor.GetComponentByClass` owner "/Game/ModsShared/AccessorySystem/Components/AC_acs_AccessorySystem.AC_acs_AccessorySystem_C") (`self.TemplateID`)))

(event `/Game/Systems/Inventory/BPGameItemEquipment.Set Stat Modifiers`
  (params (ModifierInfo :type "/Game/Systems/RiddleOfSteel/RiddleofSteelStruct Structure") (TierMultiplier :type Integer) (RemoveModifiers :type Boolean))
  (if (`self.AllowStatMods`)
    (`parent.Set Stat Modifiers` ModifierInfo TierMultiplier RemoveModifiers)))

(fn `CanBeModified`
  (params (Target :type "/Game/Systems/RiddleOfSteel/BPGameItem_RiddleOfSteel_Master Object Reference"))
  (returns (CanBeModified :type Boolean) (OutputText :type Text)))

(fn `CanItemBeDroppedOnItem`
  (params (droppedItem :type "GameItem Object Reference") (srcInventory :type "ItemInventory Object Reference") (srcIndex :type Integer))
  (returns (ReturnValue :type Boolean))
  (return false))

(fn `MakeAccessoryInfo`
  (returns (AccessoryInfo :type "/Game/ModsShared/AccessorySystem/Structs/ST_AccessoryInfo Structure"))
  (return (make `/Game/ModsShared/AccessorySystem/Structs/ST_AccessoryInfo` (`self.TemplateID`) (`self.EquipmentLocation`) (make `ArmourSlotDyeParams` (`self.GetIntStat` "DyeIndex1") (`self.GetIntStat` "DyeIndex2") (`self.GetIntStat` "DyeIndex3") (`self.GetIntStat` "DyeIndex4")) (`self.RigidAttachment`) (`self.VisualOnly`) (`self.AllowAnySlot`))))

(fn `OnItemDroppedOnItem`
  (params (droppedItem :type "GameItem Object Reference") (srcInventory :type "ItemInventory Object Reference") (srcIndex :type Integer) (controller :type "ConanPlayerController Object Reference"))
  (returns (ReturnValue :type Boolean))
  (return false))