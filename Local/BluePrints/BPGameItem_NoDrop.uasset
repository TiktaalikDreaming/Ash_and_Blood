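; Game item Blueprint for a no-drop item: it refuses moves into any inventory whose object name contains "ItemInventory", printing the target name on screen.
; It reports equip and unequip montage lengths from its VisualActor through BaseWeaponInterface, returning -1 when unavailable.
; Unequip timing prefers the EquipLength in the montage's BP_EquipMontageMetadata over the full sequence length.
; It identifies as neither armour nor projectile.
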(fn `AllowsMoveTo`
  (params (targetInventory :type "ItemInventory Object Reference"))
  (returns (ReturnValue :type Boolean))
  (bind _returnvalue (`KismetSystemLibrary.GetObjectName` targetInventory))
  (`KismetSystemLibrary.PrintString` _returnvalue true true (struct :`G` 0.66 :`B` 1.0 :`A` 1.0) 13.0)
  (if (`KismetStringLibrary.Contains` _returnvalue "ItemInventory" true)
    (return false)
    (else
      (return true))))

(fn `GetEquipItemMontageSequenceLength`
  (returns (ReturnValue :type "Float (single-precision)"))
  (bind _visualactor (`self.VisualActor`))
  (`/Engine/EditorBlueprintResources/StandardMacros.IsValid` _visualactor
    (:`Is Valid`
      (bind _asbase_weapon_interface (cast `/Game/Items/Weapons/BaseWeaponInterface` _visualactor)
        (:`then`
          (bind _value (`/Game/Items/Weapons/BaseWeaponInterface.GetItemSwapMontage` _asbase_weapon_interface))
          (`/Engine/EditorBlueprintResources/StandardMacros.IsValid` _value
            (:`Is Valid`
              (return (`AnimSequenceBase.SequenceLength` _value)))
            (:`Is Not Valid`
              _)))
        (:`CastFailed`
          _)))
    (:`Is Not Valid`
      _))
  (return -1.0))

(fn `GetUnequipItemMontageSequenceLength`
  (returns (ReturnValue :type "Float (single-precision)"))
  (bind _visualactor (`self.VisualActor`))
  (`/Engine/EditorBlueprintResources/StandardMacros.IsValid` _visualactor
    (:`Is Valid`
      (bind _asbase_weapon_interface (cast `/Game/Items/Weapons/BaseWeaponInterface` _visualactor)
        (:`then`
          (bind _value (`/Game/Items/Weapons/BaseWeaponInterface.GetItemUnequipMontage` _asbase_weapon_interface))
          (`/Engine/EditorBlueprintResources/StandardMacros.IsValid` _value
            (:`Is Valid`
              (bind _returnvalue (`FuncomGenericLibrary.GetMontageMetadata` _value "/Game/Systems/Combat/BP_EquipMontageMetadata.BP_EquipMontageMetadata_C"))
              (`/Engine/EditorBlueprintResources/StandardMacros.IsValid` _returnvalue
                (:`Is Valid`
                  (return (`/Game/Systems/Combat/BP_EquipMontageMetadata.EquipLength` _returnvalue)))
                (:`Is Not Valid`
                  (return (`AnimSequenceBase.SequenceLength` _value)))))
            (:`Is Not Valid`
              _)))
        (:`CastFailed`
          _)))
    (:`Is Not Valid`
      _))
  (return -1.0))

(fn `IsArmour`
  (returns (IsArmour :type Boolean))
  (return false))

(fn `IsProjectile`
  (returns (IsProjectile :type Boolean))
  (return false))