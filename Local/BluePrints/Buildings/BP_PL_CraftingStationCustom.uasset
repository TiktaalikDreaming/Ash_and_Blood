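; Placeable crafting station with custom GUI panels and a preservation inventory, whose recipes follow its current station ID.
; Changing the ID resets crafting groups and caches matching RecipesTable rows.
; Adding an item checks up to four ingredient quantities, but every branch breaks, so only the first cached recipe is evaluated.
; A match only prints the recipe name; activation registers the bench with the player's character component.
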(event `self.ReceiveBeginPlay`
  (`parent.ReceiveBeginPlay`)
  ;[1 0 0] Preservation box.
  (set `ItemInventory.PerishModifier` 1.0 (`self.PlaceableInventory`)))

(event `/Game/Systems/Building/Placeables/BP_Master_Placeables.ClientInteractableActivate`
  (params (Component :type "PrimitiveComponent Object Reference") (Instigator :type "PlayerController Object Reference") (HitIndex :type Integer))
  (`/Game/Mods/ash_and_blood/Actor_Components/Player/AC_BasePlayerChar.Server Set Interacted Crafting Bench` (`self.GetComponentByClass` (`Controller.K2_GetPawn` Instigator) "/Game/Mods/ash_and_blood/Actor_Components/Player/AC_BasePlayerChar.AC_BasePlayerChar_C") self))

(event `self.PlaceableInventory.SignalItemAdded`
  (params (index :type Integer) (item :type "GameItem Object Reference") (srcInventory :type "ItemInventory Object Reference") (srcIndex :type Integer))
  (`self.Check for Valid Recipe`))

(fn `Change Current Station ID`
  (params (`New ID` :type Integer))
  (bind _craftinggroups (`self.CraftingGroups`))
  (bind _output_get (set `self.CurrentStationID` `New ID`))
  (`KismetArrayLibrary.Array_Clear` _craftinggroups)
  (`KismetArrayLibrary.Array_Add` _craftinggroups _output_get)
  (`KismetArrayLibrary.Array_Clear` (`self.Valid Recipe List`))
  (bind _outrownames (`DataTableFunctionLibrary.GetDataTableRowNames` "/Game/Items/Recipes/RecipesTable.RecipesTable"))
  (for _array_element _outrownames
    (bind _returnvalue (`|GetDataTableRow` "/Game/Items/Recipes/RecipesTable.RecipesTable" _array_element)
      (:`then`
        (if (== (`.CraftingStations` (break `RecipeTableRow` _returnvalue)) (`self.CurrentStationID`))
          (`KismetArrayLibrary.Array_Add` (`self.Valid Recipe List`) _returnvalue))))))

(fn `Check for Valid Recipe`
  (locals (loc_makeRecipe :type Boolean) (loc_RecipeToMake :type "RecipeTableRow Structure"))
  (bind _placeableinventory (`self.PlaceableInventory`))
  (for _array_element (`self.Valid Recipe List`)
    (bind (_recipename _shortdesc _rank _recipetype _timetocraft _tier _craftxp _craftingstations _constructionsubclass _requiredfuel _icon _iconlayers _buildingmodule _destroystationoncomplete _recipeitemflags _ingredient1id _ingredient1quantity _ingredient2id _ingredient2quantity _ingredient3id _ingredient3quantity _ingredient4id _ingredient4quantity) (break `RecipeTableRow` _array_element))
    (if (!= _ingredient1id 0)
      (if (`ItemInventory.HasItemByTemplateID` _placeableinventory _ingredient1id _ingredient1quantity)
        (set `local.loc_makeRecipe` true)
        (if (!= _ingredient2id 0)
          (if (`ItemInventory.HasItemByTemplateID` _placeableinventory _ingredient2id _ingredient2quantity)
            (set `local.loc_makeRecipe` true)
            (if (!= _ingredient3id 0)
              (if (`ItemInventory.HasItemByTemplateID` _placeableinventory _ingredient3id _ingredient3quantity)
                (set `local.loc_makeRecipe` true)
                (if (!= _ingredient4id 0)
                  (if (`ItemInventory.HasItemByTemplateID` _placeableinventory _ingredient4id _ingredient4quantity)
                    (set `local.loc_makeRecipe` true)
                    (set `local.loc_RecipeToMake` _array_element)
                    (break)
                    (else
                      (set `local.loc_makeRecipe` false)
                      (break)))
                  (else
                    (set `local.loc_RecipeToMake` _array_element)
                    (break)))
                (else
                  (set `local.loc_makeRecipe` false)
                  (break)))
              (else
                (set `local.loc_RecipeToMake` _array_element)
                (break)))
            (else
              (set `local.loc_makeRecipe` false)
              (break)))
          (else
            (set `local.loc_RecipeToMake` _array_element)
            (break)))
        (else
          (set `local.loc_makeRecipe` false)
          (break)))
      (else
        (break))))
  (if (`local.loc_makeRecipe`)
    (`KismetSystemLibrary.PrintString` (`KismetTextLibrary.Conv_TextToString` (`.RecipeName` (break `RecipeTableRow` (`local.loc_RecipeToMake`)))))))

(fn `ClientGetCraftingGUICenterPanel`
  (params (Instigator :type "PlayerController Object Reference"))
  (returns (ReturnValue :type Name))
  (`parent.ClientGetCraftingGUICenterPanel` Instigator)
  (if (`self.Needs Custom Middle Panel`)
    (return "CustomCraftingStationInventory")
    (else
      (return "CraftingStationInventory"))))

(fn `ClientGetCraftingGUIRightPanel`
  (params (Instigator :type "PlayerController Object Reference"))
  (returns (ReturnValue :type Name))
  (`parent.ClientGetCraftingGUIRightPanel` Instigator)
  (return "CustomCraftingPanel"))

(fn `GetArtisanRecipeInventory`
  (returns (ReturnValue :type "ItemInventory Object Reference"))
  (bind _returnvalue (`parent.GetArtisanRecipeInventory`))
  (return _returnvalue))

(fn `UserConstructionScript`
  (`parent.UserConstructionScript`))