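; Placeable resource generation station that works as a crafting bench with a single active crafting group.
; On begin play it sets the inventory's perish modifier and applies its configured group ID, which replaces the crafting group list and prints a debug message.
; Client interaction registers it as the player character component's interacted bench via a server call, and the right crafting panel resolves to a custom crafting panel.
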(event `self.ReceiveBeginPlay`
  (`parent.ReceiveBeginPlay`)
  ;[1 0 0] Preservation box.
  (set `ItemInventory.PerishModifier` 1.0 (`self.PlaceableInventory`))
  (`self.Change Station Crafting Group` (`self.Crafting Group ID`)))

(event `/Game/Systems/Building/Placeables/BP_Master_Placeables.ClientInteractableActivate`
  (params (Component :type "PrimitiveComponent Object Reference") (Instigator :type "PlayerController Object Reference") (HitIndex :type Integer))
  (`/Game/Mods/ash_and_blood/Actor_Components/Player/AC_BasePlayerChar.Server Set Interacted Crafting Bench` (`self.GetComponentByClass` (`Controller.K2_GetPawn` Instigator) "/Game/Mods/ash_and_blood/Actor_Components/Player/AC_BasePlayerChar.AC_BasePlayerChar_C") self))

(fn `Change Station Crafting Group`
  (params (`Crafting Group` :type Integer))
  (bind _craftinggroups (`self.CraftingGroups`))
  (bind _output_get (set `self.Crafting Group ID` `Crafting Group`))
  (`KismetArrayLibrary.Array_Clear` _craftinggroups)
  (`KismetArrayLibrary.Array_Add` _craftinggroups _output_get)
  (`KismetSystemLibrary.PrintString` (`KismetTextLibrary.Conv_TextToString` (`|FormatText` "Crafting Gropu set to :: {iD}" _output_get))))

(fn `ClientGetCraftingGUIRightPanel`
  (params (Instigator :type "PlayerController Object Reference"))
  (returns (ReturnValue :type Name))
  (`parent.ClientGetCraftingGUIRightPanel` null)
  (return "CustomCraftingPanel"))

(fn `UserConstructionScript`
  (`parent.UserConstructionScript`))