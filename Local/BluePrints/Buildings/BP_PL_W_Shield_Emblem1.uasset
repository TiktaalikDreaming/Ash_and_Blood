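; Placeable shield building piece that displays its owning guild's emblem and can only be placed by clan members.
; On cosmetic-capable instances, BeginPlay registers a skeletal or static mesh material with GuildEmblemApplication, then sets the owning guild once the owner ID is valid or signaled.
; CanBePlaced extends the parent check with a guild test: by owner ID on the server, by the local player's character on clients.
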(event `self.ReceiveBeginPlay`
  (`parent.ReceiveBeginPlay`)
  (`/Engine/EditorBlueprintResources/StandardMacros.Can Execute Cosmetic Events`
    (:`True`
      (`GuildEmblemApplicationComponent.RegisterMaterialForGuildEmblem` (`self.GuildEmblemApplication`) (select `bool` (`self.UseSkelForEmblem`) :`false` (`self.StaticMesh`) :`true` (`self.SkeletalMesh`) :!type "PrimitiveComponent Object Reference") (`self.EmblemMaterialIndex`))
      (add `self.SignalReceivedOwnerUniqueID` (delegate `OnReceivedOwnerId`))
      (if (`StableIdFunctionLibrary.IsValidStableId` (`self.OwnerStableId`))
        (`self.OnReceivedOwnerId`)))))

(event `OnReceivedOwnerId`
  (`GuildEmblemApplicationComponent.SetOwningGuildId` (`self.GuildEmblemApplication`) (`self.OwnerStableId`)))

(fn `CanBePlaced`
  (params (AttachTo :type "BuildableBase Object Reference") (InstanceIndex :type Integer))
  (returns (FailedMessage :type String) (ReturnValue :type "ECanBePlacedResult Enum"))
  (bind (_failedmessage _returnvalue) (`parent.CanBePlaced` AttachTo InstanceIndex))
  (if (`|EnumEquality` _returnvalue "Success")
    (if (`KismetSystemLibrary.IsServer`)
      (bind _asconan_game_state (cast `ConanGameState` (`GameplayStatics.GetGameState`))
        (:`then`
          (bind _returnvalue_2 (`ConanGameState.GetServerGuildFromId` _asconan_game_state (`self.OwnerUniqueID`)))
          (if (`KismetSystemLibrary.IsValid` _returnvalue_2)
            (return "" "Success")
            (else
              _)))
        (:`CastFailed`
          _))
      (else
        (bind _asconan_player_controller (cast `ConanPlayerController` (`GameplayStatics.GetPlayerController` 0))
          (:`then`
            (if (`KismetSystemLibrary.IsValid` (`ConanCharacter.GetGuild` (`ConanPlayerController.GetConanCharacter` _asconan_player_controller)))
              (return "" "Success")
              (else
                _)))
          (:`CastFailed`
            _))))
    (return (`KismetTextLibrary.Conv_TextToString` (`self.CannotPlaceMessage`)) "Fail_NotMemberOfClan")
    (else
      (return _failedmessage _returnvalue))))

(fn `UserConstructionScript`
  (`parent.UserConstructionScript`))