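; Actor component for placeable item containers that provides bulk material storage and adjusts inventory capacity.
; On server BeginPlay, non-brush containers listed in AnB_Storage get their ItemTable slot count; unlisted ones get zero.
; When activated, it absorbs existing and newly added items, except weapons, armor and consumables, into parallel template-ID and amount arrays, deleting them from the inventory.
; A removal function decrements amounts and prunes emptied entries.
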(event `self.ReceiveBeginPlay`
  (`KismetSystemLibrary.Delay` 0.25)
  (bind _asbp_placeable_item_container (cast `/Game/Systems/Building/Placeables/BP_PlaceableItemContainer` (`self.GetOwner`)))
  (set `self.PlaceableItemContainer` _asbp_placeable_item_container)
  (if (`KismetSystemLibrary.IsServer`)
    (`self.Calculate Storage`)))

(event `MaterialStorageInventorySystem_Activate`
  (add `ItemInventory.SignalItemAdded` (`Actor.GetComponentByClass` (`self.PlaceableItemContainer`) "/Script/ConanSandbox.ItemInventoryReplicateToAll") (delegate `OnItemAddedToInventory`))
  (`self.Initial Setup of Storage`))

(event `OnItemAddedToInventory`
  (params (index :type Integer) (item :type "GameItem Object Reference") (srcInventory :type "ItemInventory Object Reference") (srcIndex :type Integer))
  (bind _stored_item (`self.Stored Item`))
  (bind _returnvalue (`GameItem.GetGUICategory` (`self.Stored Item`)))
  (bind _returnvalue_2 (`GameItem.GetIntStat` _stored_item "StackSize"))
  (bind _templateid (`GameItem.TemplateID` _stored_item))
  (bind _returnvalue_3 (`KismetArrayLibrary.Array_Find` (`self.Storage- Template ID`) _templateid))
  (set `self.Stored Item` item)
  (if (not (or (`|EnumEquality` _returnvalue "Weapon") (`|EnumEquality` _returnvalue "Armor") (`|EnumEquality` _returnvalue "Consumable")))
    (if (!= _returnvalue_3 -1)
      (`KismetArrayLibrary.Array_Set` (`self.Storage- Amounts`) _returnvalue_3 (+ (`|GetArrayItem` (`self.Storage- Amounts`) _returnvalue_3) _returnvalue_2))
      (`KismetSystemLibrary.Delay` 0.25)
      (else
        (`KismetArrayLibrary.Array_Add` (`self.Storage- Template ID`) _templateid)
        (`KismetArrayLibrary.Array_Add` (`self.Storage- Amounts`) _returnvalue_2)))
    (bind _returnvalue_4 (`ItemInventory.DeleteItemsByTemplate` (`/Game/Systems/Building/Placeables/BP_PlaceableItemContainer.PlaceableInventory` (`self.PlaceableItemContainer`)) _templateid "None" _returnvalue_2))
    (`KismetSystemLibrary.PrintString` (`KismetTextLibrary.Conv_TextToString` (`|FormatText` "Items Stored.\nItems deleted == {bool}" (select `bool` _returnvalue_4 :`false` "F" :`true` "T" :!type "Text"))))))

(fn `Calculate Storage`
  (bind _returnvalue (`Actor.GetComponentByClass` (`self.PlaceableItemContainer`) "/Script/ConanSandbox.ItemInventoryReplicateToAll"))
  (bind _returnvalue_2 (`KismetStringLibrary.Conv_StringToName` (`KismetStringLibrary.Conv_IntToString` (`BuildableBase.TemplateId` (`self.PlaceableItemContainer`)))))
  (if (not (`BuildableBase.IsABrush` (`self.PlaceableItemContainer`)))
    (bind _outrownames (`DataTableFunctionLibrary.GetDataTableRowNames` "/Game/Mods/ash_and_blood/DataTables/ControlTables/AnB_Storage.AnB_Storage"))
    (if (`KismetArrayLibrary.Array_Contains` _outrownames _returnvalue_2)
      (bind _returnvalue_3 (`|GetDataTableRow` "/Game/Items/ItemTable.ItemTable" _returnvalue_2)
        (:`then`
          (bind (_name _shortdesc _longdesc _rank _icon _iconlayers _itemclass _buildingclass _visualobject _actionblueprint_use _maxstacksize _equiplocation _guicategory _itemtags _armourvalue _armortype _soundphysicalsurface _allowsecondarymod _weapontype _weaponarchetype _compatableammunitions _soundtransmittertype _knockbackresponseweapon _weaponstaminaattacksinglebasic _weaponstaminaattacksinglespecial _weaponstaminaattackdualbasic _weaponstaminaattackdualspecial _weaponstaminaheavychargedregenmodifier _weaponspeedheavychargedmodifier _encumbranceweight _coneangle _conemaxdistance _damagehealthlight_onhit _damagehealthheavy_onhit _damagestaminalight_onhit _damagestaminaheavy_onhit _damagehealthlight_onblock _damagehealthheavy_onblock _damagestaminalight_onblock _damagestaminaheavy_onblock _harvestdamage _weaponusage _maxattackreach _minattackreach _minattackdistance _weaponeffectwidth _weaponeffectheight _itemtier _armorpen _damageconcussivelightonhit _damageconcussiveheavyonhit _damageconcussivelightonblock _damageconcussiveheavyonblock _damagetier _cooldowntime _reusetime _selectionweight _statbaseddamagetypeid _knockbackoffensebasic _knockbackoffensespecial _knockbackoffensebasiconblock _knockbackoffensespecialonblock _knockbackdefense _visualstaticmesh _visualskeletalmesh _visualdestructiblemesh _geometrycollection _weaponstatusdefault _weaponstatuscurrent _weaponstatusdecrement _perishrate _perishto _maxdurability _repairitem1 _repairitem1_amount _repairitem1_weight _repairitem2 _repairitem2_amount _repairitem2_weight _repairitem3 _repairitem3_amount _repairitem3_weight _affectedbydamagetiers _buildingpiecescore _buildingmaxhealth _repairxp _firstmodifier _secondmodifier _thirdmodifier _fourthmodifier _fifthmodifier _sixthmodifier _firstmodifiervalue _secondmodifiervalue _thirdmodifiervalue _fourthmodifiervalue _fifthmodifiervalue _sixthmodifiervalue _foodamount _drinkamount _burntime _itemflags _itemcontainersize) (break `ItemTableRow` _returnvalue_3))
          (if (!= (`ItemInventory.MaxItemCount` _returnvalue) _itemcontainersize)
            (`ItemInventory.SetMaxItemCount` _returnvalue _itemcontainersize)
            (`KismetSystemLibrary.PrintString` "Default size set.")
            (else
              (`KismetSystemLibrary.PrintString` "Is already default size.")))))
      (else
        (`ItemInventory.SetMaxItemCount` (`Actor.GetComponentByClass` (`self.PlaceableItemContainer`) "/Script/ConanSandbox.ItemInventoryReplicateToAll") 0)
        (`KismetSystemLibrary.PrintString` "Inventory set to 0.")))))

(fn `Initial Setup of Storage`
  (bind _stored_item (`self.Stored Item`))
  (bind _stored_item_2 (`self.Stored Item`))
  (bind _returnvalue (`GameItem.GetGUICategory` (`self.Stored Item`)))
  (bind _returnvalue_2 (`GameItem.GetIntStat` _stored_item "StackSize"))
  (bind _templateid (`GameItem.TemplateID` _stored_item))
  (bind _placeableinventory (`/Game/Systems/Building/Placeables/BP_PlaceableItemContainer.PlaceableInventory` (`self.PlaceableItemContainer`)))
  (bind _returnvalue_3 (`KismetArrayLibrary.Array_Find` (`self.Storage- Template ID`) _templateid))
  (bind _itemlist (`ItemInventory.ItemList` (`/Game/Systems/Building/Placeables/BP_PlaceableItemContainer.PlaceableInventory` (`self.PlaceableItemContainer`))))
  (if (> (`KismetArrayLibrary.Array_Length` _itemlist) 0)
    (for _array_element _itemlist
      (bind _output_get (set `self.Stored Item` _array_element))
      (`/Engine/EditorBlueprintResources/StandardMacros.IsValid` _output_get
        (:`Is Valid`
          (if (not (or (`|EnumEquality` _returnvalue "Weapon") (`|EnumEquality` _returnvalue "Armor") (`|EnumEquality` _returnvalue "Consumable")))
            (if (!= _returnvalue_3 -1)
              (`KismetArrayLibrary.Array_Set` (`self.Storage- Amounts`) _returnvalue_3 (+ (`|GetArrayItem` (`self.Storage- Amounts`) _returnvalue_3) _returnvalue_2))
              (else
                (`KismetArrayLibrary.Array_Add` (`self.Storage- Template ID`) _templateid)
                (`KismetArrayLibrary.Array_Add` (`self.Storage- Amounts`) _returnvalue_2)))
            (`ItemInventory.DeleteItems` _placeableinventory (`ItemInventory.GetItemIndex` _placeableinventory _stored_item_2) "None" (`GameItem.GetIntStat` _stored_item_2 "StackSize"))))))))

(fn `Remove Items from Storage`
  (params (Index :type Integer) (Amount :type Integer))
  (bind _storage__amounts (`self.Storage- Amounts`))
  (bind _output (`|GetArrayItem` _storage__amounts Index))
  (`KismetArrayLibrary.Array_Set` _storage__amounts Index (- _output Amount))
  (if (== _output 0)
    (`KismetArrayLibrary.Array_Remove` (`self.Storage- Amounts`) Index)
    (`KismetArrayLibrary.Array_Remove` (`self.Storage- Template ID`) Index)))