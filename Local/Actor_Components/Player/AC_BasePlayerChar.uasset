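; Player character component that adds server-specific building, crafting and clan rules, and makes the player immune to target lock on BeginPlay.
; Equipping the construction hammer without a clan force-unequips it with a HUD notice, and server events relay crafting station ID changes.
; Clan building and placeable caps combine member-count limits from MC_ashandBlood with donator role bonuses of clanmates in the pawn registry.
; Toggling UpdateClanUI fires its OnRep, pushing both caps to the client's guild widget.
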(event `self.ReceiveBeginPlay`
  (`self.ConstructionBeginPlay`)
  (`self.CustomAutoLockFunctionality`))

(event `Server Set Interacted Crafting Bench`
  (params (Station :type "/Game/Systems/Building/Placeables/BP_PL_Crafting_Station Object Reference"))
  (set `self.Interacted Crafting Station` Station))

(event `Server Change Current Station ID`
  (params (`New ID` :type Integer))
  (bind _asbp_pl_crafting_station_custom (cast `/Game/Mods/ash_and_blood/BluePrints/Buildings/BP_PL_CraftingStationCustom` (`self.Interacted Crafting Station`)))
  (`/Game/Mods/ash_and_blood/BluePrints/Buildings/BP_PL_CraftingStationCustom.Change Current Station ID` _asbp_pl_crafting_station_custom `New ID`))

(event `ConstructionBeginPlay`
  (`self.ToggleConstructionHammer`))

(event `ToggleConstructionHammer`
  (bind _asbase_player_char (cast `/Game/Characters/BasePlayerChar` (`self.GetOwner`)))
  (bind _output_get (set `self.BasePlayerChar` _asbase_player_char))
  (add `/Game/Characters/BaseBPCombat.SignalWeaponEquipped` _output_get (delegate `OnHammerEquipped`)))

(event `OnHammerEquipped`
  (params (Item :type "GameItem Object Reference"))
  (if (== (`GameItem.TemplateID` Item) 51033)
    (`/Engine/EditorBlueprintResources/StandardMacros.IsValid` (`ConanCharacter.GetGuild` (`self.BasePlayerChar`))
      (:`Is Not Valid`
        (`GameItem.ForceUnequip` Item)
        (`ConanCharacter.ClientHUDShowNotification` (`self.BasePlayerChar`) "You can not build without being part of a clan. Please create one, even if you are solo." true true)))))

(event `Server Calculate Storage Used`
  (bind _clan_player_count (`self.Clan Player Count`))
  (bind _baseplayerchar (`self.BasePlayerChar`))
  (bind _asbase_player_char (cast `/Game/Characters/BasePlayerChar` (`self.GetOwner`)))
  (bind _output_get (set `self.BasePlayerChar` _asbase_player_char))
  (bind _returnvalue (`ConanCharacter.GetGuild` _output_get))
  (`/Engine/EditorBlueprintResources/StandardMacros.IsValid` _returnvalue
    (:`Is Valid`
      (set `self.Clan Player Count` (- (`KismetArrayLibrary.Array_Length` (`Guild.GetGuildMembers` _returnvalue)) 1)))
    (:`Is Not Valid`
      (set `self.Clan Player Count` 0)))
  (bind _outactors (`GameplayStatics.GetAllActorsOfClass` "/Game/Mods/ash_and_blood/MC_ashandBlood.MC_ashandBlood_C"))
  (bind _output (`|GetArrayItem` _outactors))
  (set `self.Building Capacity Max` (`|GetArrayItem` (`/Game/Mods/ash_and_blood/MC_ashandBlood.Building Capacity Per Memeber` _output) _clan_player_count))
  (set `self.Placeable Capacity Max` (`|GetArrayItem` (`/Game/Mods/ash_and_blood/MC_ashandBlood.Placeable Capacity Per Memeber` _output) _clan_player_count))
  (set `self.T_BuildCap` 0)
  (set `self.T_PlaceableCap` 0)
  (bind _returnvalue_2 (`ConanWorldSettings.GetPlayerPawnRegistry` (`FuncomGenericLibrary.GetWorldSettings`)))
  (bind _returnvalue_3 (`PlayerPawnRegistry.GetPlayerPawns` _returnvalue_2))
  (for _array_element _returnvalue_3
    (bind _asbase_player_char_2 (cast `/Game/Characters/BasePlayerChar` _array_element))
    (if (!= _asbase_player_char_2 _baseplayerchar)
      (if (`/Game/Characters/BaseBPCombat.IsInSameGuild` _asbase_player_char_2 _baseplayerchar)
        (bind _donator_bonus_building_capacity (`/Game/Mods/ash_and_blood/MC_ashandBlood.Donator Bonus Building Capacity` _output))
        (bind _keys (`BlueprintMapLibrary.Map_Keys` _donator_bonus_building_capacity :!label _label))
        (for _array_element_2 _keys
          (bind _has_role (message `/Game/ModsShared/SudoExile/Auth/I_EA_AC_Player_Auth.Has Role` (`Actor.GetComponentByInterface` _asbase_player_char_2 "/Game/ModsShared/SudoExile/Auth/I_EA_AC_Player_Auth.I_EA_AC_Player_Auth_C") (`KismetStringLibrary.Conv_StringToName` _array_element_2)))
          (if _has_role
            (set `self.T_BuildCap` (`BlueprintMapLibrary.Map_Find` _donator_bonus_building_capacity _array_element_2))
            (set `self.T_PlaceableCap` (`BlueprintMapLibrary.Map_Find` (`/Game/Mods/ash_and_blood/MC_ashandBlood.Donator Bonus Placeable Capacity` _output) _array_element_2))
            (else
              (break))))
        (set `self.Building Capacity Max` (+ (`self.Building Capacity Max`) (`self.T_BuildCap`)))
        (set `self.Placeable Capacity Max` (+ (`self.Placeable Capacity Max`) (`self.T_PlaceableCap`)))
        (set `self.T_BuildCap` 0)
        (set `self.T_PlaceableCap` 0))
      (else
        (goto _label))))
  (set `self.Update Clan UI` (select `bool` (`self.Update Clan UI`) :`false` true)))

(event `CustomAutoLockFunctionality`
  (bind _asbase_player_char (cast `/Game/Characters/BasePlayerChar` (`self.GetOwner`)))
  (`/Game/Systems/Interfaces/BaseBPCharInterface.AddTargetLockImmuneReason` _asbase_player_char "ServerRestricted"))

(fn `OnRep_Update Clan UI`
  (if (not (`KismetSystemLibrary.IsServer`))
    (bind _foundwidgets (`WidgetBlueprintLibrary.GetAllWidgetsOfClass` "/Game/Mods/ash_and_blood/UserInterface/W_AAB_GuildView_UE5.W_AAB_GuildView_UE5_C"))
    (bind _output (`|GetArrayItem` _foundwidgets))
    (`/Engine/EditorBlueprintResources/StandardMacros.IsValid` _output
      (:`Is Valid`
        (`/Game/Mods/ash_and_blood/UserInterface/W_AAB_GuildView_UE5.Set StorageCapacity Used` _output 0 (`self.Building Capacity Max`) (`self.Placeable Capacity Max`) 0)))))